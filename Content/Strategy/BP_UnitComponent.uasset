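; BP_UnitComponent is a strategy-game unit component that tracks selection and shows it on the owning actor.
; SelectOverlay applies a selection overlay material to the owner's skeletal mesh and sets the UnitSelect flag; DeselectOverlay clears both.
; Click handling and AddUnitToSelectionList are empty stubs, and the owner click binding is disconnected, so selection relies on external calls to those two events.
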(event `self.ReceiveBeginPlay`)

(event `OnOwnerClicked`
  (params (TouchedActor :type "Actor Object Reference") (ButtonPressed :type "Key Structure" :default "None")))

(event `SelectOverlay`
  ;[1 1 1] Overlay On Clicked
  (`MeshComponent.SetOverlayMaterial` (`Actor.GetComponentByClass` (`self.GetOwner`) "/Script/Engine.SkeletalMeshComponent") "/Game/Material/M_OverlayForSelectUnit_Inst.M_OverlayForSelectUnit_Inst")
  (set `self.UnitSelect?` true))

(event `DeselectOverlay`
  ;[1 1 1] Overlay On Clicked
  (`MeshComponent.SetOverlayMaterial` (`Actor.GetComponentByClass` (`self.GetOwner`) "/Script/Engine.SkeletalMeshComponent") null)
  (set `self.UnitSelect?` false))

(event `AddUnitToSelectionList`)