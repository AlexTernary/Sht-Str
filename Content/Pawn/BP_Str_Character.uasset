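; BP_Str_Character is a player character pawn that can hand control back to a strategy pawn.
; Pressing Y fires BackToStr, which casts its owner to BP_PlayerControllerMain, unpossesses the character and possesses a randomly picked BP_StrPawn_2 from the level.
; It then sets Game and UI input mode and shows the mouse cursor.
; BeginPlay, Tick and overlap events are disabled stubs.
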(event `Key|Y`
  (params (Key :type "Key Structure"))
  (:`Pressed`
    (`self.BackToStr`)))

(event `BackToStr`
  (bind _as_bp_player_controller_main (`self.As BP Player Controller Main`))
  (bind _asbp_player_controller_main (cast `/Game/BP/BP_PlayerControllerMain` (`self.GetOwner`)))
  (set `self.As BP Player Controller Main` _asbp_player_controller_main)
  (`Controller.UnPossess` (`self.As BP Player Controller Main`))
  (bind _outactors (`GameplayStatics.GetAllActorsOfClass` "/Game/BP/BP_StrPawn_2.BP_StrPawn_2_C"))
  (`Controller.Possess` _as_bp_player_controller_main (`KismetArrayLibrary.Array_Random` _outactors))
  (`WidgetBlueprintLibrary.SetInputMode_GameAndUIEx` _as_bp_player_controller_main null "DoNotLock" false)
  (set `PlayerController.bShowMouseCursor` true _as_bp_player_controller_main))

(fn `UserConstructionScript`
  (`parent.UserConstructionScript`))