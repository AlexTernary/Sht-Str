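; Grenade projectile that explodes on a fixed fuse started at BeginPlay, rather than on impact.
; GranadeExplode waits out the delay, then applies radial damage at the mesh location, crediting the owner and instigator.
; ExplodeFX, commented as replicated, draws a placeholder debug sphere smaller than the damage radius and destroys the actor.
; No server check guards the damage, as the IsServer branch is unwired.
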(event `self.ReceiveBeginPlay`
  (`self.Granade Explode`))

(event `Granade Explode`
  (bind _returnvalue (`SceneComponent.K2_GetComponentLocation` (`self.StaticMesh`)))
  (`KismetSystemLibrary.Delay` 2.0)
  (`GameplayStatics.ApplyRadialDamage` 120.0 _returnvalue 1100.0 null (`|MakeArray` self :!type "Actor Object Reference") (`self.GetOwner`) (`self.GetInstigatorController`))
  (`self.Explode FX` _returnvalue))

(event `Explode FX`
  (params (Center :type "Vector Structure"))
  ;[1 1 1 1 40] Replicated explode FX
  (`KismetSystemLibrary.DrawDebugSphere` Center 800.0 12 (struct :`R` 1.0 :`G` 1.0 :`B` 1.0 :`A` 1.0) 2.0 3.0)
  (`self.K2_DestroyActor`))

(fn `UserConstructionScript`)