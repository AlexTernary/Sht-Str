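; BP_Granade is a grenade weapon Blueprint that configures the stats of an inherited weapon class.
; Its construction script sets magazine ammo before calling the parent script, then sets shooting type, damage, fire rate and total ammo.
; Fire rate is stored as a seconds-per-shot interval derived from rounds per minute.
; The event graph holds only disabled placeholder events, so the Blueprint adds no runtime logic of its own.
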(fn `UserConstructionScript`
  (set `self.Magaz Ammo` 1)
  (`parent.UserConstructionScript`)
  (set `self.Shooting Type` "NewEnumerator5")
  (set `self.Damage` 40.0)
  (set `self.Shoot Rate` (/ 1.0 (/ 60.0 60.0)))
  (set `self.Total Ammo` 7))