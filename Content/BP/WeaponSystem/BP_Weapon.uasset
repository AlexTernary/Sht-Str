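; Weapon actor that fires hitscan shots from its owning player's follow camera, in auto-rifle or single-shot mode.
; Shoot switches on ShootingType; the auto mode also sets a timer on the player's "Shoot Own" function at ShootRate before tracing.
; Both modes line-trace for objects: enemy hits spawn blood and pass Damage to the player's ShootRep, while other hits get a decal and dust effect.
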(event `Shoot`
  (switch `/Game/BP/WeaponSystem/EShooting_Type` (`self.Shooting Type`)
    (:`NewEnumerator0`
      (`self.Shoot Auto Rifle Ray`))
    (:`NewEnumerator1`
      (`self.Shoot Once Ray`))))

(event `Shoot Auto Rifle Ray`
  (bind _player (`self.Player`))
  (bind _followcamera (`/Game/ThirdPerson/Blueprints/BP_ThirdPersonCharacter.FollowCamera` _player))
  (bind _returnvalue (`SceneComponent.K2_GetComponentLocation` _followcamera))
  (`KismetSystemLibrary.K2_SetTimer` (`self.Player`) "Shoot Own" (`self.Shoot Rate`))
  (bind (_outhit _returnvalue_2) (`KismetSystemLibrary.LineTraceSingleForObjects` _returnvalue (+ _returnvalue (* (`KismetMathLibrary.GetForwardVector` (`SceneComponent.K2_GetComponentRotation` _followcamera)) 10000.0)) (`|MakeArray` "ObjectTypeQuery1" "ObjectTypeQuery4" :!type "EObjectTypeQuery Enum") false (`|MakeArray` _player :!type "Actor Object Reference") "ForOneFrame" true (struct :`R` 0.468648 :`G` 1.0 :`B` 0.990052 :`A` 0.292) (struct :`R` 0.388603 :`G` 0.910121 :`B` 1.0 :`A` 0.558) 2.0))
  (if _returnvalue_2
    (bind (_bblockinghit _binitialoverlap _time _distance _location _impactpoint _normal _impactnormal _physmat _hitactor _hitcomponent) (`GameplayStatics.BreakHitResult` _outhit))
    (bind _asbp_third_person_enemy (cast `/Game/Enemy/BP_ThirdPerson_Enemy` _hitactor)
      (:`then`
        (bind _returnvalue_3 (`KismetMathLibrary.Conv_VectorToRotator` _impactnormal))
        (bind _returnvalue_4 (* _returnvalue_3 -1.0))
        (`NiagaraFunctionLibrary.SpawnSystemAttached` "/Game/FX/FX_Blood_Spray.FX_Blood_Spray" _hitcomponent "None" _location _returnvalue_4 "KeepWorldPosition" true)
        (`/Game/ThirdPerson/Blueprints/BP_ThirdPersonCharacter.Shoot Rep` (`self.Player`) _asbp_third_person_enemy (`self.Damage`)))
      (:`CastFailed`
        (`GameplayStatics.SpawnDecalAttached` "/Game/Megascans/Decals/Round_Manhole_Cover_umeffhqcw/MI_Round_Manhole_Cover_umeffhqcw_1K.MI_Round_Manhole_Cover_umeffhqcw_1K" (9.0 9.0 9.0) _hitcomponent "None" _location _returnvalue_4 "KeepWorldPosition" 10.0)
        (`NiagaraFunctionLibrary.SpawnSystemAttached` "/Game/FX/FX_DustFromShootImpact.FX_DustFromShootImpact" _hitcomponent "None" _location _returnvalue_3 "KeepWorldPosition" true)))))

(event `Shoot Once Ray`
  (bind _player (`self.Player`))
  (bind _followcamera (`/Game/ThirdPerson/Blueprints/BP_ThirdPersonCharacter.FollowCamera` _player))
  (bind _returnvalue (`SceneComponent.K2_GetComponentLocation` _followcamera))
  (bind (_outhit _returnvalue_2) (`KismetSystemLibrary.LineTraceSingleForObjects` _returnvalue (+ _returnvalue (* (`KismetMathLibrary.GetForwardVector` (`SceneComponent.K2_GetComponentRotation` _followcamera)) 10000.0)) (`|MakeArray` "ObjectTypeQuery1" "ObjectTypeQuery4" :!type "EObjectTypeQuery Enum") false (`|MakeArray` _player :!type "Actor Object Reference") "ForOneFrame" true (struct :`R` 0.468648 :`G` 1.0 :`B` 0.990052 :`A` 0.292) (struct :`R` 0.388603 :`G` 0.910121 :`B` 1.0 :`A` 0.558) 2.0))
  (if _returnvalue_2
    (bind (_bblockinghit _binitialoverlap _time _distance _location _impactpoint _normal _impactnormal _physmat _hitactor _hitcomponent) (`GameplayStatics.BreakHitResult` _outhit))
    (bind _asbp_third_person_enemy (cast `/Game/Enemy/BP_ThirdPerson_Enemy` _hitactor)
      (:`then`
        (bind _returnvalue_3 (`KismetMathLibrary.Conv_VectorToRotator` _impactnormal))
        (bind _returnvalue_4 (* _returnvalue_3 -1.0))
        (`NiagaraFunctionLibrary.SpawnSystemAttached` "/Game/FX/FX_Blood_Spray.FX_Blood_Spray" _hitcomponent "None" _location _returnvalue_4 "KeepWorldPosition" true)
        (`/Game/ThirdPerson/Blueprints/BP_ThirdPersonCharacter.Shoot Rep` (`self.Player`) _asbp_third_person_enemy (`self.Damage`)))
      (:`CastFailed`
        (`GameplayStatics.SpawnDecalAttached` "/Game/Megascans/Decals/Round_Manhole_Cover_umeffhqcw/MI_Round_Manhole_Cover_umeffhqcw_1K.MI_Round_Manhole_Cover_umeffhqcw_1K" (9.0 9.0 9.0) _hitcomponent "None" _location _returnvalue_4 "KeepWorldPosition" 10.0)
        (`NiagaraFunctionLibrary.SpawnSystemAttached` "/Game/FX/FX_DustFromShootImpact.FX_DustFromShootImpact" _hitcomponent "None" _location _returnvalue_3 "KeepWorldPosition" true)))))

(fn `SetRefToPlayer`
  (params (Player :type "/Game/ThirdPerson/Blueprints/BP_ThirdPersonCharacter Object Reference"))
  (set `self.Player` Player))

(fn `UserConstructionScript`)