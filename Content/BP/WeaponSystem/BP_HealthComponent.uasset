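; BP_HealthComponent is an actor component that tracks hit points and regenerates them over time.
; On BeginPlay it fills current HP to max, starts a looping one-second timer and caches the owning BP_ThirdPersonCharacter.
; Each tick of that timer adds a fixed amount while HP is below max, without clamping, then sends the HP ratio to the character's OwnerController to update the HP widget.
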(event `self.ReceiveBeginPlay`
  (set `self.CurrentHP` (`self.MaxHP`))
  (`KismetSystemLibrary.K2_SetTimer` null "HP Rise" 1.0 true)
  (bind _asbp_third_person_character (cast `/Game/ThirdPerson/Blueprints/BP_ThirdPersonCharacter` (`self.GetOwner`)))
  (set `self.Charecter` _asbp_third_person_character))

(fn `HP Rise`
  (if (< (`self.CurrentHP`) (`self.MaxHP`))
    (bind _output_get (set `self.CurrentHP` (+ (`self.CurrentHP`) 4.0)))
    (bind _charecter (`self.Charecter`)
      (:`then`
        (bind _owner___controller (`/Game/ThirdPerson/Blueprints/BP_ThirdPersonCharacter.Owner - Controller` _charecter)
          (:`then`
            (`/Game/BP/BP_PC_Game.Update HP Widget` _owner___controller (/ _output_get (`self.MaxHP`))))
          (:`else`)))
      (:`else`))))