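; Game mode for a game with two player roles, shooter and "Str", providing spawn functions for each.
; Each spawn function destroys the controller's current pawn, spawns BP_ThirdPersonCharacter or BP_StrPawn_2 at a random PlayerStart, then possesses it.
; CanInStr caps Str slots by decrementing StrCount on every call and returning whether it remains non-negative.
; Nothing here calls these functions; the event graph is empty.
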(event `self.ReceiveBeginPlay`)

(fn `CanInStr?`
  (returns (Can :type Boolean))
  (bind _output_get (set `self.StrCount` (- (`self.StrCount`) 1)))
  (return (> _output_get -1)))

(fn `Find_Random_PlayerStart`
  (returns (PlayerStartTranform :type "Transform Structure (by ref)"))
  (bind _outactors (`GameplayStatics.GetAllActorsOfClass` "/Script/Engine.PlayerStart"))
  (return (`self.GetTransform` (`|GetArrayItem` _outactors (`KismetMathLibrary.RandomIntegerInRange` 0 (- (`KismetArrayLibrary.Array_Length` _outactors) 1))))))

(fn `SpawnPlayerShotter`
  (params (PlayerController :type "PlayerController Object Reference"))
  (bind _returnvalue (`Controller.K2_GetPawn` PlayerController))
  (`/Engine/EditorBlueprintResources/StandardMacros.IsValid` _returnvalue
    (:`Is Valid`
      (`self.K2_DestroyActor` _returnvalue))
    (:`Is Not Valid`
      _))
  (bind _returnvalue_2 (`|SpawnActorFromClass` "/Game/ThirdPerson/Blueprints/BP_ThirdPersonCharacter.BP_ThirdPersonCharacter_C" (`self.Find_Random_PlayerStart`) "Undefined" "OverrideRootScale" null null))
  (`Controller.Possess` PlayerController _returnvalue_2))

(fn `SpawnPlayerStr`
  (params (PlayerController :type "PlayerController Object Reference"))
  (bind _returnvalue (`Controller.K2_GetPawn` PlayerController))
  (`/Engine/EditorBlueprintResources/StandardMacros.IsValid` _returnvalue
    (:`Is Valid`
      (`self.K2_DestroyActor` _returnvalue))
    (:`Is Not Valid`
      _))
  (bind _returnvalue_2 (`|SpawnActorFromClass` "/Game/BP/BP_StrPawn_2.BP_StrPawn_2_C" (`self.Find_Random_PlayerStart`) "Undefined" "OverrideRootScale" null null))
  (`Controller.Possess` PlayerController _returnvalue_2))

(fn `UserConstructionScript`)