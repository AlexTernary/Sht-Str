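; BP_Engine is an interactable engine that builds up progress while a player interacts with it, shown on a widget component.
; Interaction start runs a looping timer that increments Progress, and interaction end clears it.
; Each tick calls ProgressMulti, apparently a multicast, which updates WB_Progress everywhere except dedicated servers.
; Progress persists between interactions, with no cap or completion logic here.
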(event `self.ReceiveBeginPlay`
  (`KismetSystemLibrary.Delay` 0.2)
  (bind _aswb_progress (cast `/Game/Widgets/WB_Progress` (`WidgetComponent.GetWidget` (`self.ProgressWidget`))))
  (`/Game/Widgets/WB_Progress.Set Progress Percent` _aswb_progress (`self.Progress`) 100.0))

(event `/Game/BP/Interaction/BPI_Interaction.InteractInterfaceCall`
  (params (WhoInteract :type "/Game/ThirdPerson/Blueprints/BP_ThirdPersonCharacter Object Reference"))
  (set `self.CanProgress` true)
  (bind _returnvalue (`KismetSystemLibrary.K2_SetTimerDelegate` (delegate `Event Progress`) 0.025 true))
  (set `self.Progress Timer` _returnvalue))

(event `/Game/BP/Interaction/BPI_Interaction.Interaction Ended`
  (set `self.CanProgress` false)
  (`KismetSystemLibrary.K2_ClearAndInvalidateTimerHandle` (`self.Progress Timer`)))

(event `Event Progress`
  (if (`self.CanProgress`)
    (set `self.Progress` (+ (`self.Progress`) 0.25))
    (`self.Event Progress Multi`)))

(event `Event Progress Multi`
  (if (not (`KismetSystemLibrary.IsDedicatedServer`))
    (bind _aswb_progress (cast `/Game/Widgets/WB_Progress` (`WidgetComponent.GetWidget` (`self.ProgressWidget`))))
    (`/Game/Widgets/WB_Progress.Set Progress Percent` _aswb_progress (`self.Progress`) 100.0)))

(fn `UserConstructionScript`)