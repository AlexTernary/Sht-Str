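; Game state Blueprint that shares pre-game timer and character characteristics with clients and opens the pre-game widgets.
; On BeginPlay it binds to the game mode's game-start event, which only prints a message.
; Setter events store RepNotify variables; minute and second notifies refresh the pre-game widget timer through the HUD cached when the widgets open.
; A lookup function maps each of three characters to its entry in the replicated characteristics array.
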(event `self.ReceiveBeginPlay`
  (bind _asbp_shoot_and_str_game_mode (cast `/Game/BP/BP_ShootAndStr_GameMode` (`GameplayStatics.GetGameMode`)))
  (add `/Game/BP/BP_ShootAndStr_GameMode.GM_Call_Game_Start` _asbp_shoot_and_str_game_mode (delegate `Game Start String`)))

(event `Game Start String`
  (`KismetSystemLibrary.PrintString` "Game Start"))

(event `Open Pre Game Widgets`
  ;[1 1 1 1 40] Open Pre Game Widget
  (`self.Replicate Open Pre Game Widgets`))

(event `Replicate Open Pre Game Widgets`
  ;[1 1 1 1 40] Open Pre Game Widget
  (bind _asbp_hud_game (cast `/Game/BP/BP_HUD_Game` (`PlayerController.GetHUD` (`GameplayStatics.GetPlayerController` 0))))
  (bind _output_get (set `self.As BP HUD Game` _asbp_hud_game))
  (`/Game/BP/BP_HUD_Game.Open PreGame Widgets` _output_get))

(event `Set Timer From Game Mode`
  (params (Minutes :type Integer) (Seconds :type Integer))
  ;[1 1 1 1 40] Replicate Timers
  (set `self.Minutes` Minutes)
  (set `self.Seconds` Seconds))

(event `Replicate Update Timer`
  ;[1 1 1 1 40] Replicate Timers
  (bind _as_bp_hud_game (`self.As BP HUD Game`)
    (:`then`
      (`/Game/Widgets/Game/WB_PreGame_Base.Update Timer` (`/Game/BP/BP_HUD_Game.WB_PreGame` _as_bp_hud_game) (`self.Minutes`) (`self.Seconds`)))
    (:`else`)))

(event `Set Pers Characteristics`
  (params (`Perss Characterirtics` :type "Array of /Game/BP/SavedData/S_Pers_Сharacteristics Structure"))
  ;[1 1 1 1 40] Replicates Perss Characteristics
  (set `self.Perss Characterirtics` `Perss Characterirtics`))

(fn `Get Pers Characteristics`
  (params (Pers :type "/Game/Characters/E_Pers_List Enum" :default "NewEnumerator0"))
  (returns (`Pers Characteristics` :type "/Game/BP/SavedData/S_Pers_Сharacteristics Structure"))
  (locals (`Pers L` :type Integer :default 0))
  (switch `/Game/Characters/E_Pers_List` Pers
    (:`NewEnumerator0`
      (set `local.Pers L` 0))
    (:`NewEnumerator1`
      (set `local.Pers L` 1))
    (:`NewEnumerator2`
      (set `local.Pers L` 2)))
  (return (`|GetArrayItem` (`self.Perss Characterirtics`) (`local.Pers L`))))

(fn `OnRep_Minutes`
  (`self.Replicate Update Timer`))

(fn `OnRep_Perss Characterirtics`
  (`KismetSystemLibrary.PrintString` "Characterictics Was Replicated" true true (struct :`R` 1.0 :`G` 1.0 :`B` 1.0 :`A` 1.0)))

(fn `OnRep_Seconds`
  (`self.Replicate Update Timer`))

(fn `UserConstructionScript`)