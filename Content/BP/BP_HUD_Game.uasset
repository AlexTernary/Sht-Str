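; Game HUD that creates and switches the pre-game, in-game and pause menu widgets, setting cursor and input mode for each.
; BeginPlay reads nickname and preferred role from BP_GI_StrShoo, applies visual settings through console commands, and calls MakeControllerStr for Str players.
; The Str flag selects the character selection widget and Str or Shoo game UI layout.
; Kill, death and statistics-list events are forwarded to the game widget.
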(event `Remove Widgets`
  (`WidgetLayoutLibrary.RemoveAllWidgets`))

(event `self.ReceiveBeginPlay`
  (bind _asbp_gi_str_shoo (cast `/Game/BP/BP_GI_StrShoo` (`GameplayStatics.GetGameInstance`)))
  (bind (_playernickname _preferrolestr_) (break `/Game/BP/SavedData/S_PlayerProfile` (`/Game/BP/BP_GI_StrShoo.Player Profile_Info` _asbp_gi_str_shoo)))
  (set `self.Player Nickname` _playernickname)
  (bind _output_get (set `self.Str?` _preferrolestr_))
  (`self.Get Visual Settings`)
  (if _output_get
    (bind _asbp_pc_game (cast `/Game/BP/BP_PC_Game` (`GameplayStatics.GetPlayerController` 0)))
    (`/Game/BP/BP_PC_Game.Make Controller Str` _asbp_pc_game)))

(event `Get Save Data`)

(event `Open PreGame Widgets`
  (bind _returnvalue (`GameplayStatics.GetPlayerController` 0))
  ;[1 1 1 1 50] Pre Game Widgets
  (set `PlayerController.bShowMouseCursor` true _returnvalue)
  (`WidgetBlueprintLibrary.SetInputMode_UIOnlyEx` _returnvalue null)
  (bind _returnvalue_2 (`|CreateWidget` "/Game/Widgets/Game/WB_PreGame_Base.WB_PreGame_Base_C" (`GameplayStatics.GetPlayerController` 0)))
  (bind _output_get (set `self.WB_PreGame` _returnvalue_2))
  (`UserWidget.AddToViewport` _output_get 0)
  (`self.Open Character Selection`))

(event `Open Character Selection`
  (bind _wb_pregame (`self.WB_PreGame`))
  (bind _wb_pregame_2 (`self.WB_PreGame`))
  ;[1 1 1 1 50] Pre Game Widgets
  (if (`self.Str?`)
    (`self.WB Character Selector`
      (:`then`
        _)
      (:`else`
        (bind _returnvalue (`|CreateWidget` "/Game/Widgets/Game/WB_Character_Selection_Str.WB_Character_Selection_Str_C" (`GameplayStatics.GetPlayerController` 0)))
        (set `self.WB Character Selector` null)))
    (`/Game/Widgets/Game/WB_PreGame_Base.Clear Child From Vertical Box` _wb_pregame_2)
    (`/Game/Widgets/Game/WB_PreGame_Base.Add Child To Vertical Box` _wb_pregame_2 _returnvalue)
    (else
      (`self.WB Character Selector`
        (:`then`
          _)
        (:`else`
          (bind _returnvalue_2 (`|CreateWidget` "/Game/Widgets/Game/WB_Character_Selection_Base.WB_Character_Selection_Base_C" (`GameplayStatics.GetPlayerController` 0)))
          (set `self.WB Character Selector` _returnvalue_2)))
      (`/Game/Widgets/Game/WB_PreGame_Base.Clear Child From Vertical Box` _wb_pregame)
      (`/Game/Widgets/Game/WB_PreGame_Base.Add Child To Vertical Box` _wb_pregame (`self.WB Character Selector`)))))

(event `Open Skills Selector`
  (params (Pers :type "/Game/Characters/E_Pers_List Enum" :default "NewEnumerator0"))
  (bind _wb_pregame (`self.WB_PreGame`))
  (bind _wb_skills_selection (`self.WB_Skills_Selection`))
  ;[1 1 1 1 50] Pre Game Widgets
  (set `self.Pers` Pers)
  (`self.WB_Skills_Selection`
    (:`then`
      _)
    (:`else`
      (bind _returnvalue (`|CreateWidget` "/Game/Widgets/Game/WB_Skills_Selection.WB_Skills_Selection_C" (`GameplayStatics.GetPlayerController` 0)))
      (set `self.WB_Skills_Selection` _returnvalue)))
  (`/Game/Widgets/Game/WB_PreGame_Base.Clear Child From Vertical Box` _wb_pregame)
  (`/Game/Widgets/Game/WB_PreGame_Base.Add Child To Vertical Box` _wb_pregame _wb_skills_selection)
  (`/Game/Widgets/Game/WB_Skills_Selection.Selected Character` _wb_skills_selection (`self.Pers`)))

(event `Game UI`
  (bind _returnvalue (`GameplayStatics.GetPlayerController` 0))
  (bind _returnvalue_2 (`GameplayStatics.GetPlayerController` 0))
  ;[1 1 1 1 50] Game Widgets
  (if (not (`self.Pause`))
    (`self.Remove Widgets`)
    (`self.WB Game`
      (:`then`
        _)
      (:`else`
        (bind _returnvalue_3 (`|CreateWidget` "/Game/Widgets/Game/WB_Game.WB_Game_C" (`GameplayStatics.GetPlayerController` 0)))
        (set `self.WB Game` _returnvalue_3)))
    (`UserWidget.AddToViewport` (`self.WB Game`) 0)
    (if (`self.Str?`)
      (`/Game/Widgets/Game/WB_Game.Set UI For Str` (`self.WB Game`))
      (set `PlayerController.bShowMouseCursor` true _returnvalue_2)
      (`WidgetBlueprintLibrary.SetInputMode_GameAndUIEx` _returnvalue_2 null "DoNotLock" false)
      (`/Game/Widgets/Game/WB_Game.Set Kills Count Widget` (`self.WB Game`) (`self.Kills`))
      (`/Engine/EditorBlueprintResources/StandardMacros.DoOnce` false
        (:`Completed`
          (`/Game/Widgets/Game/WB_Game.Create Statistic List` (`self.WB Game`))))
      (else
        (`/Game/Widgets/Game/WB_Game.Set UI For Shoo` (`self.WB Game`))
        (set `PlayerController.bShowMouseCursor` false _returnvalue)
        (`WidgetBlueprintLibrary.SetInputMode_GameOnly` _returnvalue)
        (`/Game/Widgets/Game/WB_Game.Set Kills Count Widget` (`self.WB Game`) (`self.Kills`))
        (`/Engine/EditorBlueprintResources/StandardMacros.DoOnce` false
          (:`Completed`
            (`/Game/Widgets/Game/WB_Game.Create Statistic List` (`self.WB Game`))))))))

(event `Open Pause`
  (bind _returnvalue (`GameplayStatics.GetPlayerController` 0))
  ;[1 1 1 1 40] Pause Menu
  (set `self.Pause` true)
  (`self.Remove Widgets`)
  (`self.WB Game Menu`
    (:`then`
      _)
    (:`else`
      (bind _returnvalue_2 (`|CreateWidget` "/Game/Widgets/Menus/WB_GameMenu.WB_GameMenu_C" (`GameplayStatics.GetPlayerController` 0)))
      (set `self.WB Game Menu` _returnvalue_2)))
  (`UserWidget.AddToViewport` (`self.WB Game Menu`) 0)
  (`WidgetBlueprintLibrary.SetInputMode_UIOnlyEx` _returnvalue null)
  (set `PlayerController.bShowMouseCursor` true _returnvalue))

(event `Set Pause`
  (params (Pause :type Boolean))
  ;[1 1 1 1 40] Pause Menu
  (set `self.Pause` Pause))

(event `Set Kills`
  (params (Kills :type "Float (double-precision)"))
  ;[1 1 1 1 40] Info About Players
  (set `self.Kills` Kills)
  (bind _wb_game (`self.WB Game`)
    (:`then`
      (`/Game/Widgets/Game/WB_Game.Set Kills Count Widget` _wb_game (`self.Kills`)))
    (:`else`)))

(event `Set Deaths`
  (params (Deaths :type "Float (double-precision)"))
  ;[1 1 1 1 40] Info About Players
  (set `self.Deaths` Deaths)
  (bind _wb_game (`self.WB Game`)
    (:`then`
      (`/Game/Widgets/Game/WB_Game.Set Deaths Count Widget` _wb_game (`self.Deaths`)))
    (:`else`)))

(event `Create Statisctic List`
  ;[1 1 1 1 40] Info About All Players
  (bind _wb_game (`self.WB Game`)
    (:`then`
      (`/Game/Widgets/Game/WB_Game.Create Statistic List` _wb_game))
    (:`else`)))

(event `Add Kills`
  (params (Kills :type "Array of Float (double-precision)"))
  ;[1 1 1 1 40] Info About All Players
  (bind _wb_game (`self.WB Game`)
    (:`then`
      (`/Game/Widgets/Game/WB_Game.Add Kills` _wb_game Kills))
    (:`else`)))

(event `Add Deaths`
  (params (Deaths :type "Array of Float (double-precision)"))
  ;[1 1 1 1 40] Info About All Players
  (bind _wb_game (`self.WB Game`)
    (:`then`
      (`/Game/Widgets/Game/WB_Game.Add Deaths` _wb_game Deaths))
    (:`else`)))

(fn `Get Visual Settings`
  (bind _asbp_gi_str_shoo (cast `/Game/BP/BP_GI_StrShoo` (`GameplayStatics.GetGameInstance`)))
  (`|ExecutionSequence`
    (:`then_0`
      (bind (_volumetric_fog _anti_alisingmethod _motionblur) (break `/Game/BP/SavedData/S_Visual_Settings` (`/Game/BP/BP_GI_StrShoo.Visual Settings` _asbp_gi_str_shoo)))
      (if _volumetric_fog
        (`KismetSystemLibrary.ExecuteConsoleCommand` "r.VolumetricFog 1" (`GameplayStatics.GetPlayerController` 0))
        (else
          (`KismetSystemLibrary.ExecuteConsoleCommand` "r.VolumetricFog 0" (`GameplayStatics.GetPlayerController` 0)))))
    (:`then_1`
      (switch `int` _anti_alisingmethod
        (:`0`
          (`KismetSystemLibrary.ExecuteConsoleCommand` "r.AntiAliasingMethod 0" (`GameplayStatics.GetPlayerController` 0)))
        (:`1`
          (`KismetSystemLibrary.ExecuteConsoleCommand` "r.AntiAliasingMethod 1" (`GameplayStatics.GetPlayerController` 0)))
        (:`2`
          (`KismetSystemLibrary.ExecuteConsoleCommand` "r.AntiAliasingMethod 2" (`GameplayStatics.GetPlayerController` 0)))
        (:`3`
          (`KismetSystemLibrary.ExecuteConsoleCommand` "r.AntiAliasingMethod 3" (`GameplayStatics.GetPlayerController` 0)))))
    (:`then_2`
      (if _motionblur
        (`KismetSystemLibrary.ExecuteConsoleCommand` "r.MotionBlurQuality 1" (`GameplayStatics.GetPlayerController` 0))
        (else
          (`KismetSystemLibrary.ExecuteConsoleCommand` "r.MotionBlurQuality 0" (`GameplayStatics.GetPlayerController` 0)))))
    (:`then_3`
      (`KismetSystemLibrary.ExecuteConsoleCommand` "sg.GlobalIlluminationQuality 1" (`GameplayStatics.GetPlayerController` 0)))))

(fn `UserConstructionScript`)