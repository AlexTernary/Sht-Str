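; AI controller for the enemy bot in the shooter/strategy game.
; On possessing a BP_ThirdPerson_Enemy, it runs the BI_AI_Bot behavior tree.
; On BeginPlay it binds to the game mode's SpawnInStrRepCall dispatcher, which makes the strategy player controller the owner of this AI controller.
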(event `self.ReceivePossess`
  (params (PossessedPawn :type "Pawn Object Reference"))
  (cast `/Game/Enemy/BP_ThirdPerson_Enemy` PossessedPawn)
  (`self.RunBehaviorTree` "/Game/BP/Strategy/BI_AI_Bot.BI_AI_Bot"))

(event `self.ReceiveBeginPlay`
  (bind _asbp_shoot_and_str_game_mode (cast `/Game/BP/BP_ShootAndStr_GameMode` (`GameplayStatics.GetGameMode`)))
  (add `/Game/BP/BP_ShootAndStr_GameMode.SpawnInStrRepCall` _asbp_shoot_and_str_game_mode (delegate `SetNewOwner`)))

(event `SetNewOwner`
  (`self.SetOwner` (`/Game/BP/BP_ShootAndStr_GameMode.Player Controller Str` (stale `self.ReceiveBeginPlay` _asbp_shoot_and_str_game_mode))))

(fn `UserConstructionScript`)