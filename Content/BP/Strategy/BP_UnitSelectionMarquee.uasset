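; World-space drag-selection marquee for picking units in a strategy game.
; Each mouse hit moves the end corner, re-centring and resizing a tall collision box between it and the actor's location.
; While the mouse is held, overlap begin and end send select and deselect messages to BPI_UnitSelector actors and the player controller.
; Box collision turns on only after a brief hold, and release disables it and hides the marquee.
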(event `self.ReceiveBeginPlay`
  (`self.SetActorHiddenInGame` false))

(event `/Game/BP/Strategy/BPI_MouseLocationHit.MouseLocationHit`
  (params (MouseLocationHit :type "Vector Structure"))
  (bind (_returnvalue_x _returnvalue_y _returnvalue_z) (`KismetMathLibrary.BreakVector` (`KismetMathLibrary.VLerp` (`self.K2_GetActorLocation`) (`self.EndBoxLocation`) 0.5)))
  (bind (_returnvalue_x_2 _returnvalue_y_2) (`KismetMathLibrary.BreakVector` (/ (`KismetMathLibrary.Vector_GetAbs` (- (`self.EndBoxLocation`) (`self.K2_GetActorLocation`))) 2.0)))
  (bind _output_get (set `self.EndBoxLocation` MouseLocationHit))
  (`SceneComponent.K2_SetWorldLocation` (`self.Sphere`) _output_get false true)
  (`SceneComponent.K2_SetWorldLocation` (`self.BoxSelection`) (`KismetMathLibrary.MakeVector` _returnvalue_x _returnvalue_y (+ _returnvalue_z -100.0)) false false)
  (`SceneComponent.K2_SetWorldLocation` (`self.Sphere2`) (`KismetMathLibrary.MakeVector` _returnvalue_x _returnvalue_y (+ _returnvalue_z -100.0)) false false)
  (`BoxComponent.SetBoxExtent` (`self.BoxSelection`) (`KismetMathLibrary.MakeVector` _returnvalue_x_2 _returnvalue_y_2 500.0) true))

(event `self.BoxSelection.OnComponentBeginOverlap`
  (params (OverlappedComponent :type "PrimitiveComponent Object Reference") (OtherActor :type "Actor Object Reference") (OtherComp :type "PrimitiveComponent Object Reference") (OtherBodyIndex :type Integer) (bFromSweep :type Boolean) (SweepResult :type "HitResult Structure (by ref)"))
  (if (`self.Mouse Down`)
    (if (`KismetSystemLibrary.DoesImplementInterface` OtherActor "/Game/BP/Strategy/BPI_UnitSelector.BPI_UnitSelector_C")
      (message `/Game/BP/Strategy/BPI_UnitSelector.SelectThisActor` (`GameplayStatics.GetPlayerController` 0) OtherActor)
      (message `/Game/BP/Strategy/BPI_UnitSelector.SelectThisActor` OtherActor null))))

(event `self.BoxSelection.OnComponentEndOverlap`
  (params (OverlappedComponent :type "PrimitiveComponent Object Reference") (OtherActor :type "Actor Object Reference") (OtherComp :type "PrimitiveComponent Object Reference") (OtherBodyIndex :type Integer))
  (if (`self.Mouse Down`)
    (if (`KismetSystemLibrary.DoesImplementInterface` OtherActor "/Game/BP/Strategy/BPI_UnitSelector.BPI_UnitSelector_C")
      (message `/Game/BP/Strategy/BPI_UnitSelector.DeselectThisActor` OtherActor null)
      (message `/Game/BP/Strategy/BPI_UnitSelector.DeselectThisActor` (`GameplayStatics.GetPlayerController` 0) OtherActor))))

(event `/Game/BP/Strategy/BPI_MouseLocationHit.MouseDown`
  (params (MouseDown :type Boolean))
  (bind _boxselection (`self.BoxSelection`))
  (bind _output_get (set `self.Mouse Down` MouseDown))
  (if _output_get
    (`KismetSystemLibrary.Delay` 0.1)
    (if (`self.Mouse Down`)
      (`PrimitiveComponent.SetCollisionEnabled` _boxselection "QueryOnly")
      (`self.SetActorHiddenInGame` false))
    (else
      (`PrimitiveComponent.SetCollisionEnabled` _boxselection "NoCollision")
      (`self.SetActorHiddenInGame` true))))

(fn `UserConstructionScript`)