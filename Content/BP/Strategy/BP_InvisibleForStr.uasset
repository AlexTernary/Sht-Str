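; BP_InvisibleForStr is a component that hides its owning actor, apparently a ceiling, while the player is in strategy (Str) control.
; On BeginPlay it casts player controller 0 to BP_PlayerControllerMain and binds HideCelling to its SpawnInStr event.
; When fired on a local controller, HideCelling sets the owner hidden or visible from IsStrController, leaving collision untouched.
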(event `self.ReceiveBeginPlay`
  (bind _asbp_player_controller_main (cast `/Game/BP/BP_PlayerControllerMain` (`GameplayStatics.GetPlayerController` 0)))
  (add `/Game/BP/BP_PlayerControllerMain.SpawnInStr` _asbp_player_controller_main (delegate `Hide Celling`)))

(event `Hide Celling`
  (bind _returnvalue (`self.GetOwner`))
  (if (`Controller.IsLocalController` (`GameplayStatics.GetPlayerController` 0))
    (if (`/Game/BP/BP_PlayerControllerMain.IsStrController?` (stale `self.ReceiveBeginPlay` _asbp_player_controller_main))
      (`Actor.SetActorHiddenInGame` _returnvalue true)
      (else
        (`Actor.SetActorHiddenInGame` _returnvalue false)))))