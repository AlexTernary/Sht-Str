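; Menu game state that relays lobby player info and map changes, with naming and comments indicating replication to all clients.
; Player info from the game mode is stored, then passed to the lobby widget through the local player's menu HUD.
; Map changes go through a Rep-to-Multi event pair that calls either MapUp or MapDown based on a direction flag.
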(event `self.ReceiveBeginPlay`)

(event `Get Player Info From Game Mode`
  (params (`Info Of All Players` :type "Array of /Game/BP/SavedData/S_PlayerProfile Structure"))
  ;[1 1 1 1 40] Replicates save info from game mode to all clients
  (`self.Replicate Player Connected To Clients` `Info Of All Players`))

(event `Replicate Player Connected To Clients`
  (params (`Info Of All Players` :type "Array of /Game/BP/SavedData/S_PlayerProfile Structure"))
  ;[1 1 1 1 40] Replicates save info from game mode to all clients
  (set `self.Info Of All Players` `Info Of All Players`)
  (bind _asbp_hud_menu (cast `/Game/BP/BP_HUD_Menu` (`PlayerController.GetHUD` (`GameplayStatics.GetPlayerController` 0))))
  (`/Game/Widgets/Session/WB_Lobby.Get Player Info From Game State` (`/Game/BP/BP_HUD_Menu.WB Lobby` _asbp_hud_menu) (`self.Info Of All Players`)))

(event `Map_Change_Rep`
  (params (`Up?` :type Boolean))
  (`self.Map_Change_Multi` `Up?`))

(event `Map_Change_Multi`
  (params (`Up?` :type Boolean))
  (if `Up?`
    (`self.MapUp`)
    (else
      (`self.MapDown`))))

(fn `UserConstructionScript`)