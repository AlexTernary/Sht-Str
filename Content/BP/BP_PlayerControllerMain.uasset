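; Player controller for a hybrid shooter and strategy game that lets a local player pick a role through a spawn widget.
; The game mode spawns a strategist if allowed, otherwise a shooter, and the controller sets matching UI and input.
; Strategists right-click to send selected units to the cursor hit; interface events maintain the selection, while left-click marquee logic is disconnected.
; The L key destroys the session and returns to the main menu.
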(event `self.ReceiveBeginPlay`
  (bind _asbp_shoot_and_str_game_mode (cast `/Game/BP/BP_ShootAndStr_GameMode` (`GameplayStatics.GetGameMode`))
    (:`then`
      (set `self.As BP Shoot And Str Game Mode` _asbp_shoot_and_str_game_mode))
    (:`CastFailed`
      _))
  (if (`self.IsLocalPlayerController`)
    (bind _returnvalue (`|CreateWidget` "/Game/Widgets/WB_SpawnInStr.WB_SpawnInStr_C"))
    (set `self.SpawnWidget` _returnvalue)
    (`UserWidget.AddToViewport` _returnvalue 0)
    (set `self.bShowMouseCursor` true)
    (`WidgetBlueprintLibrary.SetInputMode_UIOnlyEx` self (`self.SpawnWidget`))))

(event `Spawn Own`
  (params (`IsStrController?` :type Boolean))
  (`self.SR_SpawnPlayer` `IsStrController?`))

(event `SR_SpawnPlayer`
  (params (`IsStrController?` :type Boolean))
  ;[1 1 1 1 40] Spawn
  (if `IsStrController?`
    (bind _can (`/Game/BP/BP_ShootAndStr_GameMode.CanInStr?` (`self.As BP Shoot And Str Game Mode`)))
    (if _can
      (`self.Create Game UI` true)
      (`/Game/BP/BP_ShootAndStr_GameMode.SpawnPlayerStr` (`self.As BP Shoot And Str Game Mode`) self)
      (set `self.bShowMouseCursor` true)
      (set `self.bEnableClickEvents` true)
      (else
        (`self.Create Game UI` false :!label _label)
        (`/Game/BP/BP_ShootAndStr_GameMode.SpawnPlayerShotter` (`self.As BP Shoot And Str Game Mode`) self)))
    (else
      (goto _label))))

(event `Create Game UI`
  (params (Condition :type Boolean))
  ;[1 1 1] Game UI
  (set `self.IsStrController?` Condition)
  (bind _spawnwidget (`self.SpawnWidget`)
    (:`then`
      (`Widget.RemoveFromParent` _spawnwidget))
    (:`else`
      _))
  (if (`self.IsLocalPlayerController`)
    (if (`self.IsStrController?`)
      (`WidgetBlueprintLibrary.SetInputMode_GameAndUIEx` self null "DoNotLock" false)
      (`self.SpawnInStr`)
      (else
        (`self.AddShotterUI`)))))

(event `AddActorToSelected`
  (params (SelectedActor :type "Actor Object Reference"))
  ;[1 1 1] Add Selected
  (`KismetArrayLibrary.Array_Add` (`self.SelectedActor`) SelectedActor))

(event `DeselectAllActors`
  ;[1 1 1] Deselect All
  (for _array_element (`self.SelectedActor`)
    (if (`KismetSystemLibrary.DoesImplementInterface` _array_element "/Game/BP/Strategy/BPI_UnitSelector.BPI_UnitSelector_C")
      (message `/Game/BP/Strategy/BPI_UnitSelector.DeselectThisActor` _array_element null)))
  (`KismetArrayLibrary.Array_Clear` (`self.SelectedActor`)))

(event `EnhancedInput|/Game/ThirdPerson/Input/Actions/IA_RightClick`
  (params (ActionValue :type Boolean) (ElapsedSeconds :type "Float (double-precision)") (TriggeredSeconds :type "Float (double-precision)") (InputAction :type "InputAction Object Reference" :default "/Game/ThirdPerson/Input/Actions/IA_RightClick.IA_RightClick"))
  ;[1 1 1] Right Mouse
  (:`Started`
    (if (`self.IsStrController?`)
      (if (`KismetArrayLibrary.Array_IsNotEmpty` (`self.SelectedActor`))
        (bind _output_get (set `self.Location` (`.Location` (`GameplayStatics.BreakHitResult` (`self.GetHitResultUnderCursorByChannel` "TraceTypeQuery1")))))
        (`KismetSystemLibrary.DrawDebugSphere` _output_get 80.0 12 (struct :`R` 1.0 :`G` 0.456088 :`B` 0.426232 :`A` 1.0) 0.5 3.0)
        (`self.UpdateGoalLocation Rep` (`self.SelectedActor`) _output_get)))))

(event `UpdateGoalLocation Rep`
  (params (Array :type "Array of Actor Object Reference") (Destination :type "Vector Structure"))
  ;[1 1 1] Right Mouse
  ;;[1 1 1] Unit Movement
  (for _array_element Array
    (bind _asbp_third_person_enemy (cast `/Game/Enemy/BP_ThirdPerson_Enemy` _array_element))
    (`/Game/Enemy/BP_ThirdPerson_Enemy.NewTargetLocation Rep` _asbp_third_person_enemy Destination)))

(event `EnhancedInput|/Game/ThirdPerson/Input/Actions/IA_LeftClick`
  (params (ActionValue :type Boolean) (ElapsedSeconds :type "Float (double-precision)") (TriggeredSeconds :type "Float (double-precision)") (InputAction :type "InputAction Object Reference" :default "/Game/ThirdPerson/Input/Actions/IA_LeftClick.IA_LeftClick"))
  ;[1 1 1] Left Mouse
)

(event `/Game/BP/Strategy/BPI_UnitSelector.SelectThisActor`
  (params (ActorSelected :type "Actor Object Reference"))
  ;[1 1 1] Interface Selector
  (`self.AddActorToSelected` ActorSelected))

(event `/Game/BP/Strategy/BPI_UnitSelector.DeselectThisActor`
  (params (ActorDeselected :type "Actor Object Reference"))
  ;[1 1 1] Interface Selector
  (`KismetArrayLibrary.Array_RemoveItem` (`self.SelectedActor`) ActorDeselected))

(event `Key|L`
  (params (Key :type "Key Structure"))
  (:`Pressed`
    (`DestroySessionCallbackProxy.DestroySession` (`GameplayStatics.GetPlayerController` 0)
      (:`OnSuccess`
        (`GameplayStatics.OpenLevel` "MainMenu"))
      (:`OnFailure`
        (`KismetSystemLibrary.PrintString` "Can't destroy" true true (struct :`R` 1.0 :`G` 0.093511 :`B` 0.113406 :`A` 1.0) 12.0)
        (`GameplayStatics.OpenLevel` "MainMenu")))))

(fn `AddShotterUI`
  (if (`self.IsLocalController`)
    (bind _returnvalue (`|CreateWidget` "/Game/Widgets/WB_GameSht.WB_GameSht_C" self))
    (`UserWidget.AddToViewport` _returnvalue 0)
    (`KismetSystemLibrary.PrintString` (`KismetSystemLibrary.GetDisplayName` _returnvalue))
    (`WidgetBlueprintLibrary.SetInputMode_GameOnly` self)
    (set `self.bShowMouseCursor` false)))

(fn `AddStrUI`)

(fn `SelectOneActor`
  (bind (_bblockinghit _binitialoverlap _time _distance _location _impactpoint _normal _impactnormal _physmat _hitactor) (`GameplayStatics.BreakHitResult` (`self.GetHitResultUnderCursorByChannel` "TraceTypeQuery3")))
  (`self.DeselectAllActors`)
  (if (`KismetSystemLibrary.DoesImplementInterface` _hitactor "/Game/BP/Strategy/BPI_UnitSelector.BPI_UnitSelector_C")
    (message `/Game/BP/Strategy/BPI_UnitSelector.SelectThisActor` _hitactor null)
    (`self.AddActorToSelected` _hitactor)
    (return)
    (else
      (return))))

(fn `UserConstructionScript`)