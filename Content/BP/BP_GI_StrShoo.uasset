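; Game instance for a multiplayer shooter that manages LAN sessions, level travel, top-level UI and the saved player profile.
; Events create or destroy the lobby session and servertravel to maps by console command.
; Menu, search, settings and shooter HUD widgets are cached on first use and swapped by clearing all widgets, with some setting input mode.
; Nickname and preferred role persist through an SG_PlayerProfile save slot, checked when the main menu opens.
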(event `Create Lobby`
  ;[1 1 1 1 40] Create Lobby
  (`CreateSessionCallbackProxy.CreateSession` (`GameplayStatics.GetPlayerController` 0) 5 true
    (:`OnSuccess`
      (`GameplayStatics.OpenLevel` "Lobby_1" true "listen"))))

(event `SearchForLobbyWidget`
  ;[1 1 1 1 40] Search Lobby Widget
  (`WidgetLayoutLibrary.RemoveAllWidgets`)
  (`self.WB_FindSession`
    (:`then`
      _)
    (:`else`
      (bind _returnvalue (`|CreateWidget` "/Game/Widgets/Session/WB_SearchSession.WB_SearchSession_C" (`GameplayStatics.GetPlayerController` 0)))
      (bind _output_get (set `self.WB_FindSession` _returnvalue))))
  (`UserWidget.AddToViewport` _output_get 0))

(event `TravelToMap`
  (params (NumberOfConectedPlayers :type Integer) (Map :type String))
  ;[1 1 1 1 40] Travel To Game Level
  (set `self.Number Of Conected Players` NumberOfConectedPlayers)
  (`KismetSystemLibrary.ExecuteConsoleCommand` (`KismetStringLibrary.Concat_StrStr` "servertravel " Map) (`GameplayStatics.GetPlayerController` 0)))

(event `MainMenuWidgets`
  (bind (_playernickname _preferrolestr_) (break `/Game/BP/SavedData/S_PlayerProfile` (`self.Player Profile_Info`)))
  (bind _wb_playerprofile (`/Game/Widgets/Menus/WB_MainMenu.WB_PlayerProfile` (`self.WB_MainMenu`)))
  ;[1 1 1 1 40] Main Menu Widget
  (if (not (`KismetSystemLibrary.IsDedicatedServer`))
    (`WidgetLayoutLibrary.RemoveAllWidgets`)
    (`self.WB_MainMenu`
      (:`then`
        _)
      (:`else`
        (bind _returnvalue (`|CreateWidget` "/Game/Widgets/Menus/WB_MainMenu.WB_MainMenu_C" (`GameplayStatics.GetPlayerController` 0)))
        (set `self.WB_MainMenu` _returnvalue)))
    (`UserWidget.AddToViewport` (`self.WB_MainMenu`) 0)
    (`WidgetBlueprintLibrary.SetInputMode_GameAndUIEx` (`GameplayStatics.GetPlayerController` 0) null "LockInFullscreen" false)
    (`self.CheckForSavedProfile`)
    (`/Game/Widgets/Menus/WB_PlayerProfile.SetNickname_Text` _wb_playerprofile _playernickname)
    (`/Game/Widgets/Menus/WB_PlayerProfile.Set Prefer Role` _wb_playerprofile _preferrolestr_)))

(event `Destroy Lobby`
  ;[1 1 1 1 40] Leave Lobby
  (if (`KismetSystemLibrary.IsServer`)
    (`DestroySessionCallbackProxy.DestroySession` (`GameplayStatics.GetPlayerController` 0)
      (:`then`
        (`KismetSystemLibrary.PrintString` "Destr" true true (struct :`R` 0.979 :`G` 0.99286 :`B` 1.0 :`A` 1.0))
        (`GameplayStatics.OpenLevel` "MainMenu")))
    (else
      (`DestroySessionCallbackProxy.DestroySession` (`GameplayStatics.GetPlayerController` 0)
        (:`OnSuccess`
          (`GameplayStatics.OpenLevel` "MainMenu")
          (`KismetSystemLibrary.Delay` 0.01)
          (`self.SearchForLobbyWidget`))))))

(event `Open Settings`
  (params (InMainMenu :type Boolean))
  (bind _wb_settings (`self.WB_Settings`))
  ;[1 1 1 1 40] Open Settings
  (set `self.InMainMenu` InMainMenu)
  (`WidgetLayoutLibrary.RemoveAllWidgets`)
  (`self.WB_Settings`
    (:`then`
      _)
    (:`else`
      (bind _returnvalue (`|CreateWidget` "/Game/Widgets/Menus/WB_Settings.WB_Settings_C" (`GameplayStatics.GetPlayerController` 0)))
      (set `self.WB_Settings` _returnvalue)))
  (`UserWidget.AddToViewport` _wb_settings 0)
  (set `/Game/Widgets/Menus/WB_Settings.IsInMainMenu?` (`self.InMainMenu`) _wb_settings))

(event `MenuInGame`
  (bind _returnvalue (`GameplayStatics.GetPlayerController` 0))
  ;[1 1 1 1 40] Game Menu
  (if (not (`KismetSystemLibrary.IsDedicatedServer`))
    (`WidgetLayoutLibrary.RemoveAllWidgets`)
    (`self.WB_GameMenu`
      (:`then`
        _)
      (:`else`
        (bind _returnvalue_2 (`|CreateWidget` "/Game/Widgets/Menus/WB_GameMenu.WB_GameMenu_C" (`GameplayStatics.GetPlayerController` 0)))
        (set `self.WB_GameMenu` _returnvalue_2)))
    (`UserWidget.AddToViewport` (`self.WB_GameMenu`) 0)
    (`WidgetBlueprintLibrary.SetInputMode_UIOnlyEx` _returnvalue null)
    (set `PlayerController.bShowMouseCursor` true _returnvalue)))

(event `Change Nckname`
  (params (Nickname :type Text))
  ;[1 1 1 1 40] Check SaveData
  (set `self.Player Profile_Info` (make `/Game/BP/SavedData/S_PlayerProfile` Nickname (`.PreferRoleStr?_5_A527D2C6488C16386F46909C54886419` (break `/Game/BP/SavedData/S_PlayerProfile` (`self.Player Profile_Info`)))))
  (`self.SaveProfile`))

(event `Change Prefer Role`
  (params (`PreferRoleStr?` :type Boolean))
  ;[1 1 1 1 40] Check SaveData
  (set `self.Player Profile_Info` (make `/Game/BP/SavedData/S_PlayerProfile` (`.PlayerNickname_2_0C8C4B62483BE247FBB029B66046D3CF` (break `/Game/BP/SavedData/S_PlayerProfile` (`self.Player Profile_Info`))) `PreferRoleStr?`))
  (`self.SaveProfile`))

(fn `CheckForSavedProfile`
  (bind _returnvalue (`GameplayStatics.DoesSaveGameExist` (`self.PlayerProfile_Slot`)))
  (if _returnvalue
    (bind _assg_player_profile (`self.LoadProfile`))
    (set `self.SG Player Profile` _assg_player_profile)
    (else
      (`self.SaveProfile`)))
  (return))

(fn `Create ShooterUI`
  (returns (`Shoo UI` :type "/Game/Widgets/WB_GameSht Object Reference"))
  (bind _returnvalue (`GameplayStatics.GetPlayerController` 0))
  (`WidgetLayoutLibrary.RemoveAllWidgets`)
  (`self.Shoo UI`
    (:`then`
      _)
    (:`else`
      (bind _returnvalue_2 (`|CreateWidget` "/Game/Widgets/WB_GameSht.WB_GameSht_C" (`GameplayStatics.GetPlayerController` 0)))
      (set `self.Shoo UI` _returnvalue_2)))
  (`UserWidget.AddToViewport` (`self.Shoo UI`) 0)
  (`WidgetBlueprintLibrary.SetInputMode_GameOnly` _returnvalue)
  (set `PlayerController.bShowMouseCursor` false _returnvalue)
  (return (`self.Shoo UI`)))

(fn `LoadProfile`
  (returns (`AsSG Player Profile` :type "/Game/BP/SavedData/SG_PlayerProfile Object Reference"))
  (bind _returnvalue (`GameplayStatics.LoadGameFromSlot` (`self.PlayerProfile_Slot`)))
  (bind _assg_player_profile (cast `/Game/BP/SavedData/SG_PlayerProfile` _returnvalue))
  (set `self.Player Profile_Info` (`/Game/BP/SavedData/SG_PlayerProfile.PlayerProfile` _assg_player_profile))
  (return _assg_player_profile))

(fn `SaveProfile`
  (bind _sg_player_profile (`self.SG Player Profile`))
  (`self.SG Player Profile`
    (:`then`
      _)
    (:`else`
      (bind _returnvalue (`GameplayStatics.CreateSaveGameObject` "/Game/BP/SavedData/SG_PlayerProfile.SG_PlayerProfile_C"))
      (set `self.SG Player Profile` _returnvalue)))
  (set `/Game/BP/SavedData/SG_PlayerProfile.PlayerProfile` (`self.Player Profile_Info`) _sg_player_profile)
  (`GameplayStatics.SaveGameToSlot` _sg_player_profile (`self.PlayerProfile_Slot`))
  (return))