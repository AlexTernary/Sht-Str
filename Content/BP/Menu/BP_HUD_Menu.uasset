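; Menu HUD Blueprint that shows level-specific UI when play begins.
; It switches on the current level name, and for "Lobby 1" creates WB_Lobby for player controller 0, reusing the stored instance if valid, and adds it to the viewport.
; An event meant to bind to BP_GS_Menu's PlayerConnected is unfinished: it only casts the game state, and the bind node never runs.
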(event `self.ReceiveBeginPlay`
  (`self.Switch On Levels`))

(event `Switch On Levels`
  ;[1 1 1] Create Widgets Dependet On Current Level
  (bind _returnvalue (`GameplayStatics.GetCurrentLevelName` true))
  (switch `string` _returnvalue
    (:`Lobby_1`
      (`self.Create Lobby Widget`))))

(event `Create Lobby Widget`
  ;[1 1 1] Manage Lobby Widgets
  (`self.WB Lobby`
    (:`then`
      _)
    (:`else`
      (bind _returnvalue (`|CreateWidget` "/Game/Widgets/Lobby/WB_Lobby.WB_Lobby_C" (`GameplayStatics.GetPlayerController` 0)))
      (set `self.WB Lobby` _returnvalue)))
  (`UserWidget.AddToViewport` (`self.WB Lobby`) 0))

(event `Bing 'Player Connected' From Game State`
  ;[1 1 1] Manage Lobby Widgets
  (bind _asbp_gs_menu (cast `/Game/BP/Menu/BP_GS_Menu` (`GameplayStatics.GetGameState`))))

(fn `UserConstructionScript`)