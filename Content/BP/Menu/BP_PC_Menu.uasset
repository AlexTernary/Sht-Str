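; Menu player controller that carries the player's profile (nickname and preferred role) between the game instance and the main menu and lobby.
; On BeginPlay it loads the saved profile, and role changes update the game instance and game mode.
; Paired forwarding events pass level opening to the game mode and map switching to the game state.
; It can refill the lobby player list, but widget creation and list-gathering logic are disconnected.
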(event `self.ReceiveBeginPlay`
  (`self.Get Save Data`))

(event `Get Save Data`
  ;[1 1 1 1 40] Get save data and replicate it to game mode
  (bind _asbp_gi_str_shoo (cast `/Game/BP/BP_GI_StrShoo` (`GameplayStatics.GetGameInstance`)))
  (`self.Replicate Saved Data` (`/Game/BP/BP_GI_StrShoo.Player Profile_Info` _asbp_gi_str_shoo)))

(event `Replicate Saved Data`
  (params (`Player Info` :type "/Game/BP/SavedData/S_PlayerProfile Structure"))
  ;[1 1 1 1 40] Get save data and replicate it to game mode
  (set `self.Player Info` `Player Info`))

(event `Change Role`
  (bind (_playernickname _preferrolestr_) (break `/Game/BP/SavedData/S_PlayerProfile` (`self.Player Info`)))
  (bind _returnvalue (not _preferrolestr_))
  ;[1 1 1 1 40] Get save data and replicate it to game mode
  (bind _output_get (set `self.Player Info` (make `/Game/BP/SavedData/S_PlayerProfile` _playernickname _returnvalue)))
  (bind _asbp_gi_str_shoo (cast `/Game/BP/BP_GI_StrShoo` (`GameplayStatics.GetGameInstance`)))
  (`/Game/BP/BP_GI_StrShoo.Change Prefer Role` _asbp_gi_str_shoo _returnvalue)
  (`self.Replicate Saved Data` _output_get)
  (`self.Update Data In Game Mode`))

(event `Update Data In Game Mode`
  ;[1 1 1 1 40] Get save data and replicate it to game mode
  (bind _asbp_gm_main_menu (cast `/Game/BP/BP_GM_MainMenu` (`GameplayStatics.GetGameMode`)))
  (`/Game/BP/BP_GM_MainMenu.Update Save Data` _asbp_gm_main_menu))

(event `OpenMainMaenu`)

(event `Open Lobby Widget`
  ;[1 1 1 1 40] Lobby Widget
)

(event `Open Level 1`
  ;[1 1 1 1 40] Open level 1
  (`self.Open Level 1 Rep`))

(event `Open Level 1 Rep`
  ;[1 1 1 1 40] Open level 1
  (bind _asbp_gm_main_menu (cast `/Game/BP/BP_GM_MainMenu` (`GameplayStatics.GetGameMode`)))
  (`/Game/BP/BP_GM_MainMenu.Open Level 1 GM` _asbp_gm_main_menu))

(event `Replicate Button In Lobby`
  (params (`MapUp?` :type Boolean))
  ;[1 1 1 1 40] Replicates Button Lobby
  (`self.Replicate Buttom In Lobby 2` `MapUp?`))

(event `Replicate Buttom In Lobby 2`
  (params (`Map Up?` :type Boolean))
  ;[1 1 1 1 40] Replicates Button Lobby
  (bind _asbp_gs_menu (cast `/Game/BP/Menu/BP_GS_Menu` (`GameplayStatics.GetGameState`)))
  (`/Game/BP/Menu/BP_GS_Menu.Map_Change_Rep` _asbp_gs_menu `Map Up?`))

(event `Replicate Saved Info`)

(event `Replicate Saved Info 2`)

(event `Replicate Saved Info 3`
  (params (`Profile Info` :type "Array of /Game/BP/SavedData/S_PlayerProfile Structure"))
  (bind _wb_lobby (`self.WB_Lobby`)
    (:`then`
      (`/Game/Widgets/Session/WB_Lobby.Clear Player Lists` _wb_lobby)
      (for _array_element `Profile Info`
        (bind _wb_lobby_2 (`self.WB_Lobby`)
          (:`then`
            (bind (_playernickname _preferrolestr_) (break `/Game/BP/SavedData/S_PlayerProfile` _array_element))
            (`/Game/Widgets/Session/WB_Lobby.AddPlayerToList` _wb_lobby_2 _playernickname _preferrolestr_))
          (:`else`))))
    (:`else`)))

(fn `Get Saved Info`
  (returns (`Player Profile_Info` :type "/Game/BP/SavedData/S_PlayerProfile Structure"))
  (return (`self.Player Info`)))

(fn `Set Player NickName`
  (params (PlayerNickname :type Text))
  (set `self.Player Info` (make `/Game/BP/SavedData/S_PlayerProfile` PlayerNickname (`.PreferRoleStr?_5_A527D2C6488C16386F46909C54886419` (break `/Game/BP/SavedData/S_PlayerProfile` (`self.Player Info`))))))

(fn `Set Player Role`
  (params (`PreferRoleStr?` :type Boolean))
  (set `self.Player Info` (make `/Game/BP/SavedData/S_PlayerProfile` (`.PlayerNickname_2_0C8C4B62483BE247FBB029B66046D3CF` (break `/Game/BP/SavedData/S_PlayerProfile` (`self.Player Info`))) `PreferRoleStr?`)))

(fn `UserConstructionScript`)