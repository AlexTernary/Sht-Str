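; Main menu game mode that tracks players joining and leaving the Lobby 1 level and shares their saved player info.
; After a short post-login delay it stores each menu player controller, and on logout it removes it.
; Each change rebuilds the info array from all controllers, passes it to BP_GS_Menu and copies it into BP_GI_StrShoo.
; A helper gathers saved info from every controller, while level-travel nodes are left unconnected.
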(event `Open Level 1 GM`)

(event `self.HandleStartingNewPlayer`
  (params (NewPlayer :type "PlayerController Object Reference")))

(event `Update Save Data`
  ;[1 1 1 1 40] Get All Player Conntroller And Replicate Save Data From Them To Game State
  (`KismetArrayLibrary.Array_Clear` (`self.Info Of All Players`))
  (for _array_element (`self.AllConectedPlayerController`)
    (`KismetArrayLibrary.Array_Add` (`self.Info Of All Players`) (`/Game/BP/Menu/BP_PC_Menu.Player Info` _array_element)))
  (bind _asbp_gs_menu (cast `/Game/BP/Menu/BP_GS_Menu` (`GameplayStatics.GetGameState`)))
  (`/Game/BP/Menu/BP_GS_Menu.Get Player Info From Game Mode` _asbp_gs_menu (`self.Info Of All Players`)))

(event `self.K2_PostLogin`
  (params (NewPlayer :type "PlayerController Object Reference"))
  ;[1 1 1 1 40] Get All Player Conntroller And Replicate Save Data From Them To Game State
  (`KismetSystemLibrary.Delay` 0.2)
  (bind _asbp_pc_menu (cast `/Game/BP/Menu/BP_PC_Menu` NewPlayer)
    (:`then`
      (bind _returnvalue (`GameplayStatics.GetCurrentLevelName` true))
      (switch `string` _returnvalue
        (:`Lobby_1`
          (`KismetArrayLibrary.Array_Add` (`self.AllConectedPlayerController`) _asbp_pc_menu)
          (`self.Update Save Data`)
          (`self.Transfer Saved Data` (`self.Info Of All Players`)))))
    (:`CastFailed`
      (`KismetSystemLibrary.PrintString` "Cast PC Faild"))))

(event `self.K2_OnLogout`
  (params (ExitingController :type "Controller Object Reference"))
  ;[1 1 1 1 40] Get All Player Conntroller And Replicate Save Data From Them To Game State
  (bind _asbp_pc_menu (cast `/Game/BP/Menu/BP_PC_Menu` ExitingController)
    (:`then`
      (bind _returnvalue (`KismetArrayLibrary.Array_RemoveItem` (`self.AllConectedPlayerController`) _asbp_pc_menu))
      (if _returnvalue
        (`self.Update Save Data`)
        (`self.Transfer Saved Data` (`self.Info Of All Players`))))
    (:`CastFailed`
      (`KismetSystemLibrary.PrintString` "Cast PC Faild"))))

(event `Transfer Saved Data`
  (params (`Info Of All Players` :type "Array of /Game/BP/SavedData/S_PlayerProfile Structure"))
  ;[1 1 1 1 40] Get All Player Conntroller And Replicate Save Data From Them To Game State
  (bind _asbp_gi_str_shoo (cast `/Game/BP/BP_GI_StrShoo` (`GameplayStatics.GetGameInstance`)))
  (set `/Game/BP/BP_GI_StrShoo.Info Of All Players` `Info Of All Players` _asbp_gi_str_shoo))

(fn `Get Saved Info For All`
  (returns (`Player Info` :type "Array of /Game/BP/SavedData/S_PlayerProfile Structure"))
  (locals (`Player Info L` :type "Array of /Game/BP/SavedData/S_PlayerProfile Structure"))
  (for _array_element (`self.AllConectedPlayerController`)
    (bind _player_profile_info (`/Game/BP/Menu/BP_PC_Menu.Get Saved Info` _array_element))
    (`KismetArrayLibrary.Array_Add` (`local.Player Info L`) _player_profile_info))
  (return (`local.Player Info L`)))

(fn `UserConstructionScript`)