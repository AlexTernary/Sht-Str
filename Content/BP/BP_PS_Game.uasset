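; BP_PS_Game is the game's player state, tracking each player's kill and death counts.
; CountKills and CountDeaths add a whole point when the Player flag is set and a tenth otherwise, then send the total to the HUD through the player controller.
; OnRep functions rebuild kill and death arrays by looping over player states and pass them to the first controller's HUD.
; GetKillsFromAll is an empty stub.
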(event `Count Kills`
  (params (`Player?` :type Boolean))
  ;[1 1 1 1 40] Count Kills And Deaths
  (if `Player?`
    (bind _output_get (set `self.Kills` (+ (`self.Kills`) 1.0)))
    (`self.Replicate Kills To All ` _output_get)
    (else
      (bind _output_get_2 (set `self.Kills` (+ (`self.Kills`) 0.1)))
      (`self.Replicate Kills To All ` _output_get_2))))

(event `Replicate Kills To All`
  (params (Kills :type "Float (double-precision)"))
  ;[1 1 1 1 40] Count Kills And Deaths
  (bind _asbp_pc_game (cast `/Game/BP/BP_PC_Game` (`self.GetPlayerController`)))
  (bind _asbp_hud_game (cast `/Game/BP/BP_HUD_Game` (`PlayerController.GetHUD` _asbp_pc_game)))
  (`/Game/BP/BP_HUD_Game.Set Kills` _asbp_hud_game Kills))

(event `REplicate Deaths To All`
  (params (Deaths :type "Float (double-precision)"))
  ;[1 1 1 1 40] Count Kills And Deaths
  (bind _asbp_pc_game (cast `/Game/BP/BP_PC_Game` (`self.GetPlayerController`)))
  (bind _asbp_hud_game (cast `/Game/BP/BP_HUD_Game` (`PlayerController.GetHUD` _asbp_pc_game)))
  (`/Game/BP/BP_HUD_Game.Set Deaths` _asbp_hud_game Deaths))

(event `Count Deaths`
  (params (Player :type Boolean))
  ;[1 1 1 1 40] Count Kills And Deaths
  (if Player
    (bind _output_get (set `self.Deaths` (+ (`self.Deaths`) 1.0)))
    (`self.REplicate Deaths To All` _output_get)
    (else
      (bind _output_get_2 (set `self.Deaths` (+ (`self.Deaths`) 0.1)))
      (`self.REplicate Deaths To All` _output_get_2))))

(event `Get Kills From All`)

(fn `OnRep_Deaths`
  (`KismetArrayLibrary.Array_Clear` (`self.All Deaths`))
  (for _index (range (+ (`GameplayStatics.GetNumPlayerControllers`) 1))
    (bind _asbp_ps_game (cast `/Game/BP/BP_PS_Game` (`GameplayStatics.GetPlayerState` _index)))
    (`KismetArrayLibrary.Array_Add` (`self.All Deaths`) (`/Game/BP/BP_PS_Game.Deaths` _asbp_ps_game)))
  (bind _asbp_hud_game (cast `/Game/BP/BP_HUD_Game` (`PlayerController.GetHUD` (`GameplayStatics.GetPlayerController` 0))))
  (`/Game/BP/BP_HUD_Game.Add Deaths` _asbp_hud_game (`self.All Deaths`)))

(fn `OnRep_Kills`
  (`KismetArrayLibrary.Array_Clear` (`self.All Kills`))
  (for _index (range (+ (`GameplayStatics.GetNumPlayerControllers`) 1))
    (bind _asbp_ps_game (cast `/Game/BP/BP_PS_Game` (`GameplayStatics.GetPlayerState` _index)))
    (`KismetArrayLibrary.Array_Add` (`self.All Kills`) (`/Game/BP/BP_PS_Game.Kills` _asbp_ps_game)))
  (bind _asbp_hud_game (cast `/Game/BP/BP_HUD_Game` (`PlayerController.GetHUD` (`GameplayStatics.GetPlayerController` 0))))
  (`/Game/BP/BP_HUD_Game.Add Kills` _asbp_hud_game (`self.All Kills`)))

(fn `UserConstructionScript`)