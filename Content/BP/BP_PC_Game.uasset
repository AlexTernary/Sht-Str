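; Player controller for a game where each player is either a shooter or a strategy ("Str") commander.
; Role choice and spawning go through BP_ShootAndStr_GameMode, with input mode, cursor and shooter HP UI set per role.
; Strategy right-click sends selected enemy units to the cursor hit, tracked via BPI_UnitSelector, though click and marquee selection are unwired.
; Also handles pause menu and session exit, while respawn and win/loss handlers mostly just print.
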(event `self.ReceiveBeginPlay`
  (bind _asbp_shoot_and_str_game_mode (cast `/Game/BP/BP_ShootAndStr_GameMode` (`GameplayStatics.GetGameMode`)))
  (set `self.As BP Shoot And Str Game Mode` _asbp_shoot_and_str_game_mode)
  (`self.Bind Game End`))

(event `Respawn`
  ;[1 1 1 1 40] Create Where To Spawn Widgets (Old)
  (`KismetSystemLibrary.PrintString` "PC Should Respawn"))

(event `Spawn Own`
  (params (`IsStrController?` :type Boolean))
  (`self.SR_SpawnPlayer` `IsStrController?`))

(event `SR_SpawnPlayer`
  (params (`IsStrController?` :type Boolean))
  ;[1 1 1 1 40] Spawn (Old)
  (`/Game/BP/BP_ShootAndStr_GameMode.GM_Call_PlayerConnect` (`self.As BP Shoot And Str Game Mode`))
  (if `IsStrController?`
    (bind _can (`/Game/BP/BP_ShootAndStr_GameMode.CanInStr?` (`self.As BP Shoot And Str Game Mode`)))
    (if _can
      (`self.Add Game UI` true)
      (`/Game/BP/BP_ShootAndStr_GameMode.SpawnPlayerStr` (`self.As BP Shoot And Str Game Mode`) self)
      (set `self.bShowMouseCursor` true)
      (set `self.bEnableClickEvents` true)
      (`/Game/BP/BP_ShootAndStr_GameMode.TransferControllerId` (`self.As BP Shoot And Str Game Mode`))
      (`self.MultiCallSpawnInStr`)
      (else
        (`self.Add Game UI` false :!label _label)
        (bind _controledplayer (`/Game/BP/BP_ShootAndStr_GameMode.SpawnPlayerShotter` (`self.As BP Shoot And Str Game Mode`) self))
        (bind _bp_healthcomponent (`/Game/ThirdPerson/Blueprints/BP_ThirdPersonCharacter.BP_HealthComponent` _controledplayer))
        (bind _maxhp (`/Game/BP/WeaponSystem/BP_HealthComponent.MaxHP` _bp_healthcomponent))
        (bind _output_get (set `/Game/BP/WeaponSystem/BP_HealthComponent.CurrentHP` _maxhp _bp_healthcomponent))
        (`KismetSystemLibrary.Delay` 0.1)
        (`self.Update HP Widget` (/ _output_get _maxhp))))
    (else
      (goto _label))))

(event `Add Game UI`
  (params (Condition :type Boolean))
  ;[1 1 1 1 40] Game UI
  (set `self.IsStrController?` Condition)
  (`WidgetLayoutLibrary.RemoveAllWidgets`)
  (if (`self.IsLocalPlayerController`)
    (if (`self.IsStrController?`)
      (`WidgetBlueprintLibrary.SetInputMode_GameAndUIEx` self null "DoNotLock" false)
      (else
        (`self.Shoo UI`)))))

(event `MultiCallSpawnInStr`
  ;[1 1 1 1 40] Spawn (Old)
  (`self.SpawnInStr`))

(event `Shoo UI`
  (bind _asbp_gi_str_shoo (cast `/Game/BP/BP_GI_StrShoo` (`GameplayStatics.GetGameInstance`)))
  (bind _shoo_ui (`/Game/BP/BP_GI_StrShoo.Create ShooterUI` _asbp_gi_str_shoo))
  (set `self.Sht Widgets` _shoo_ui))

(event `AddActorToSelected`
  (params (SelectedActor :type "Actor Object Reference"))
  ;[1 1 1 1 40] Add Selected
  (`KismetArrayLibrary.Array_Add` (`self.SelectedActor`) SelectedActor))

(event `DeselectAllActors`
  ;[1 1 1 1 40] Deselect All
  (for _array_element (`self.SelectedActor`)
    (if (`KismetSystemLibrary.DoesImplementInterface` _array_element "/Game/BP/Strategy/BPI_UnitSelector.BPI_UnitSelector_C")
      (message `/Game/BP/Strategy/BPI_UnitSelector.DeselectThisActor` _array_element null)))
  (`KismetArrayLibrary.Array_Clear` (`self.SelectedActor`)))

(event `EnhancedInput|/Game/ThirdPerson/Input/Actions/IA_RightClick`
  (params (ActionValue :type Boolean) (ElapsedSeconds :type "Float (double-precision)") (TriggeredSeconds :type "Float (double-precision)") (InputAction :type "InputAction Object Reference" :default "/Game/ThirdPerson/Input/Actions/IA_RightClick.IA_RightClick"))
  ;[1 1 1 1 40] Right Mouse
  (:`Started`
    (if (`self.IsStrController?`)
      (if (`KismetArrayLibrary.Array_IsNotEmpty` (`self.SelectedActor`))
        (bind _output_get (set `self.Location` (`.Location` (`GameplayStatics.BreakHitResult` (`self.GetHitResultUnderCursorByChannel` "TraceTypeQuery1")))))
        (`KismetSystemLibrary.DrawDebugSphere` _output_get 80.0 12 (struct :`R` 1.0 :`G` 0.456088 :`B` 0.426232 :`A` 1.0) 0.5 3.0)
        (`self.UpdateGoalLocation Rep` (`self.SelectedActor`) _output_get)))))

(event `UpdateGoalLocation Rep`
  (params (Array :type "Array of Actor Object Reference") (Destination :type "Vector Structure"))
  ;[1 1 1 1 40] Right Mouse
  ;;[1 1 1] Unit Movement
  (for _array_element Array
    (bind _asbp_third_person_enemy (cast `/Game/Enemy/BP_ThirdPerson_Enemy` _array_element))
    (`/Game/Enemy/BP_ThirdPerson_Enemy.NewTargetLocation Rep` _asbp_third_person_enemy Destination)))

(event `EnhancedInput|/Game/ThirdPerson/Input/Actions/IA_LeftClick`
  (params (ActionValue :type Boolean) (ElapsedSeconds :type "Float (double-precision)") (TriggeredSeconds :type "Float (double-precision)") (InputAction :type "InputAction Object Reference" :default "/Game/ThirdPerson/Input/Actions/IA_LeftClick.IA_LeftClick"))
  ;[1 1 1 1 40] Left Mouse
)

(event `/Game/BP/Strategy/BPI_UnitSelector.SelectThisActor`
  (params (ActorSelected :type "Actor Object Reference"))
  ;[1 1 1 1 40] Interface Selector
  (`self.AddActorToSelected` ActorSelected))

(event `/Game/BP/Strategy/BPI_UnitSelector.DeselectThisActor`
  (params (ActorDeselected :type "Actor Object Reference"))
  ;[1 1 1 1 40] Interface Selector
  (`KismetArrayLibrary.Array_RemoveItem` (`self.SelectedActor`) ActorDeselected))

(event `Key|L`
  (params (Key :type "Key Structure"))
  ;[1 1 1 1 41] Leave Session
)

(event `Leave Session`
  ;[1 1 1 1 41] Leave Session
  (`DestroySessionCallbackProxy.DestroySession` (`GameplayStatics.GetPlayerController` 0)
    (:`OnSuccess`
      _)
    (:`OnFailure`
      (`KismetSystemLibrary.PrintString` "Can't destroy" true true (struct :`R` 1.0 :`G` 0.093511 :`B` 0.113406 :`A` 1.0))))
  (`GameplayStatics.OpenLevel` "MainMenu"))

(event `Respawn Event`
  ;[1 1 1 1 40] Respawn
  (`WidgetLayoutLibrary.RemoveAllWidgets`)
  (`self.Respawn`))

(event `Update HP Widget`
  (params (`Percent HP` :type "Float (double-precision)"))
  ;[1 1 1 1 40] Update HP Widget
  (`KismetSystemLibrary.PrintString` (`KismetStringLibrary.Concat_StrStr` "HP  " (`KismetStringLibrary.Conv_DoubleToString` `Percent HP`)) true true (struct :`R` 1.0 :`G` 1.0 :`B` 1.0 :`A` 1.0))
  (bind _sht_widgets (`self.Sht Widgets`)
    (:`then`
      (`/Game/Widgets/Game/WB_GameSht.Set HP ` _sht_widgets `Percent HP`))
    (:`else`)))

(event `Key|P`
  (params (Key :type "Key Structure"))
  ;[1 1 1 1 40] Pause Game
  (:`Pressed`
    (bind _asbp_gi_str_shoo (cast `/Game/BP/BP_GI_StrShoo` (`GameplayStatics.GetGameInstance`)))
    (`/Game/BP/BP_GI_StrShoo.MenuInGame` _asbp_gi_str_shoo)))

(event `Bind Game End`
  (add `/Game/BP/BP_ShootAndStr_GameMode.StrWin` (`self.As BP Shoot And Str Game Mode`) (delegate `Replicates Str Win`))
  (add `/Game/BP/BP_ShootAndStr_GameMode.ShooWin` (`self.As BP Shoot And Str Game Mode`) (delegate `Replicates Shoo Win`)))

(event `Replicates Str Win`
  (`KismetSystemLibrary.PrintString` "Loose" true true (struct :`R` 1.0 :`G` 0.025124 :`A` 1.0) 5.0))

(event `Replicates Shoo Win`
  (`KismetSystemLibrary.PrintString` "Win" true true (struct :`R` 0.017098 :`G` 1.0 :`A` 1.0) 5.0))

(event `Set Pers From UI`
  (params (Pers :type "/Game/Characters/E_Pers_List Enum" :default "NewEnumerator0"))
  ;[1 1 1 1 41] Replicate Chosen Pers and 'Ready' to Game Mode
  (`self.Replicate Pers and Ready to Game Mode` Pers)
  (switch `/Game/Characters/E_Pers_List` Pers
    (:`NewEnumerator0`
      (`WidgetBlueprintLibrary.SetInputMode_GameOnly` self :!label _label_2)
      (set `self.bShowMouseCursor` false)
      (`self.Shoo UI`))
    (:`NewEnumerator1`
      (goto _label_2))
    (:`NewEnumerator2`
      (goto _label_2))
    (:`NewEnumerator3`
      (set `self.bShowMouseCursor` true)
      (`WidgetBlueprintLibrary.SetInputMode_GameAndUIEx` self null "DoNotLock" false))))

(event `Replicate Pers and Ready to Game Mode`
  (params (Pers :type "/Game/Characters/E_Pers_List Enum" :default "NewEnumerator0"))
  ;[1 1 1 1 41] Replicate Chosen Pers and 'Ready' to Game Mode
  (set `self.Pers` Pers)
  (bind _asbp_shoot_and_str_game_mode (cast `/Game/BP/BP_ShootAndStr_GameMode` (`GameplayStatics.GetGameMode`)))
  (`/Game/BP/BP_ShootAndStr_GameMode.Set Chosen Pers` _asbp_shoot_and_str_game_mode (`self.Pers`) self))

(event `Make Controller Str`
  ;[1 1 1 1 41] Replicate Chosen Pers and 'Ready' to Game Mode
  (`self.Make Controller Str Replicated`)
  (`self.SpawnInStr`))

(event `Make Controller Str Replicated`
  ;[1 1 1 1 41] Replicate Chosen Pers and 'Ready' to Game Mode
  (set `self.IsStrController?` true))

(fn `AddShotterUI`
  (if (`self.IsLocalController`)
    (bind _returnvalue (`|CreateWidget` "/Game/Widgets/Game/WB_GameSht.WB_GameSht_C" self))
    (bind _output_get (set `self.Sht Widgets` _returnvalue))
    (`UserWidget.AddToViewport` _output_get 0)
    (`KismetSystemLibrary.PrintString` (`KismetSystemLibrary.GetDisplayName` _returnvalue))
    (`WidgetBlueprintLibrary.SetInputMode_GameOnly` self)
    (set `self.bShowMouseCursor` false)))

(fn `AddStrUI`)

(fn `SelectOneActor`
  (bind (_bblockinghit _binitialoverlap _time _distance _location _impactpoint _normal _impactnormal _physmat _hitactor) (`GameplayStatics.BreakHitResult` (`self.GetHitResultUnderCursorByChannel` "TraceTypeQuery3")))
  (`self.DeselectAllActors`)
  (if (`KismetSystemLibrary.DoesImplementInterface` _hitactor "/Game/BP/Strategy/BPI_UnitSelector.BPI_UnitSelector_C")
    (message `/Game/BP/Strategy/BPI_UnitSelector.SelectThisActor` _hitactor null)
    (`self.AddActorToSelected` _hitactor)
    (return)
    (else
      (return))))

(fn `UserConstructionScript`)